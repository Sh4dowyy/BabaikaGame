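; AI enemy character that spots the player and performs a melee catch attack.
; Pawn sensing sets the blackboard's seeingPlayer flag for Player-tagged pawns, while a looping timer periodically clears it; hearing only prints a debug string.
; CatchPlayer plays a guarded montage and sphere-traces from CatchTracePoint to apply damage.
; The trace end multiplies location by the forward offset, and damage reads a hit-array loop that never executes.
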(event OnSeePawn(PawSensing)
  (params (Pawn :type Pawn%20Object%20Reference))
  (if (Actor|ActorHasTag Pawn "Player")
    (AI|Components|Blackboard|SetValueasBool (AI|GetBlackboard (AI|GetAIController self)) (Utilities|Name|MakeLiteralName "seeingPlayer") true)))

(event OnHearNoise(PawSensing)
  (params (Instigator :type Pawn%20Object%20Reference) (Location :type Vector%20%28by%20ref%29 :default "0, 0, 0") (Volume :type Float%20%28single-precision%29))
  (Development|PrintString "Hello"))

(event Custom|Catch%20Player
  (bind _catch_trace_point (Variables|Default|GetCatch%20Trace%20Point))
  (bind _returnvalue (Transformation|GetWorldLocation _catch_trace_point))
  (if (not (Variables|Default|Getattacking))
    (Variables|Default|Setattacking true)
    (Animation|Montage|PlayMontage (Variables|Character|GetMesh) "/Game/AI/AM_Caught.AM_Caught"
      (:then
        (bind (_outhits _returnvalue_2) (Collision|MultiSphereTraceForObjects _returnvalue (* _returnvalue (* (Math|Vector|GetForwardVector (Transformation|GetWorldRotation _catch_trace_point)) 7e+01)) 25.0 (Utilities|Array|MakeArray "ObjectTypeQuery3") false 0 "None"))
        (if _returnvalue_2
          (Game|Damage|ApplyDamage (.HitActor (Collision|BreakHitResult (stale _array_element))) 1e+01 0 0)))
      (:OnCompleted
        (Variables|Default|Setattacking false)))))

(event Custom|Stop%20Scene%20Layer
  ;[0.15 0.15 0.15 0.5] Escape From Enemys Sight
  (AI|Components|Blackboard|SetValueasBool (AI|GetBlackboard (AI|GetAIController self)) (Utilities|Name|MakeLiteralName "seeingPlayer") false))

(event EventBeginPlay
  ;[0.15 0.15 0.15 0.5] Escape From Enemys Sight
  (Utilities|Time|SetTimerbyEvent (delegate Custom|Stop%20Scene%20Layer) 0.8 true))

(fn ConstructionScript)